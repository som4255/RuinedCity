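; BP_커브배치 is a spline placement actor that lays copies of a chosen static mesh (배치될메시) along a curve.
; Its construction script derives the spacing from the mesh's X bounds plus a gap (메시간거리), then sets the count from spline length.
; GetLocationIndex converts each index into a local spline position, where an InstancedStaticMesh instance is added with X aimed at the next point.
; The event graph is empty.
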(fn `Get Location Index`
  (params (A :type "Float (double-precision)"))
  (returns (ReturnValue :type "Vector Structure"))
  (return (`SplineComponent.GetLocationAtDistanceAlongSpline` (`self.Spline`) (* A (`self.메시간 배치거리`)) "Local")))

(fn `UserConstructionScript`
  (locals (`인스턴스 수` :type Integer))
  (bind (_min _max) (break `Box` (`StaticMesh.GetBoundingBox` (`self.배치될 메시`))))
  (`StaticMeshComponent.SetStaticMesh` (`self.InstancedStaticMesh`) (`self.배치될 메시`))
  (bind _output_get (set `self.메시간 배치거리` (+ (.x (- _max _min)) (`self.메시간 거리`))))
  (bind _output_get_2 (set `local.인스턴스 수` (`KismetMathLibrary.Conv_Int64ToInt` (`KismetMathLibrary.FFloor64` (/ (`SplineComponent.GetSplineLength` (`self.Spline`)) _output_get)))))
  (for _index (range (+ _output_get_2 1))
    (bind _returnvalue (`self.Get Location Index` (`KismetMathLibrary.Conv_IntToDouble` _index)))
    (`InstancedStaticMeshComponent.AddInstance` (`self.InstancedStaticMesh`) (`KismetMathLibrary.MakeTransform` _returnvalue (`KismetMathLibrary.MakeRotFromX` (- (`self.Get Location Index` (`KismetMathLibrary.Conv_IntToDouble` (+ _index 1))) _returnvalue))) false)))