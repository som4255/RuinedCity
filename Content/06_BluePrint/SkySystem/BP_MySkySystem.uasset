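; Sky system actor that drives a time-of-day sun and a switchable rainy weather look.
; Tick advances TimeOfDay by TimeSpeed, maps it to directional light pitch, and rewrites two rain Material Parameter Collections from the Rainy flag.
; The construction script previews sun angle and weather, including fog density, MSRain visibility and light intensity.
; SetRainy and SetUnRainy switch those weather settings without changing Rainy, so Tick overrides their collection values.
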(event `self.ReceiveTick`
  (params (DeltaSeconds :type "Float (single-precision)"))
  (`SceneComponent.K2_SetWorldRotation` (`self.DirectionalLight`) (`KismetMathLibrary.MakeRotator` 0.0 (`KismetMathLibrary.MapRangeUnclamped` (`self.TimeOfDay`) 600.0 1800.0 180.0 360.0) (`self.SunAngle`)) false false)
  (set `self.TimeOfDay` (+ (`self.TimeOfDay`) (* DeltaSeconds (`self.TimeSpeed`))))
  (if (`self.Rainy`)
    (`KismetMaterialLibrary.SetScalarParameterValue` "/Game/07_RainyWeather/MPC_Rainy.MPC_Rainy" "RippleFlatten")
    (`KismetMaterialLibrary.SetScalarParameterValue` "/Game/17_NiagaraEffect/NiagaraSystem/Rain/RainMaterialEffect/MPC_Rain.MPC_Rain" "Rain" 1.0)
    (else
      (`KismetMaterialLibrary.SetScalarParameterValue` "/Game/07_RainyWeather/MPC_Rainy.MPC_Rainy" "RippleFlatten" 1.0)
      (`KismetMaterialLibrary.SetScalarParameterValue` "/Game/17_NiagaraEffect/NiagaraSystem/Rain/RainMaterialEffect/MPC_Rain.MPC_Rain" "Rain"))))

(event `SetRainy`
  (`self.SetRain`))

(event `SetUnRainy`
  (`self.SetUnRain`))

(event `Test`
  (`KismetSystemLibrary.PrintString` "Hello"))

(fn `SetRain`
  (`KismetMaterialLibrary.SetScalarParameterValue` "/Game/07_RainyWeather/MPC_Rainy.MPC_Rainy" "RippleFlatten")
  (`ExponentialHeightFogComponent.SetFogDensity` (`self.ExponentialHeightFog`) 0.3)
  (`SceneComponent.SetVisibility` (`self.MS_Rain`) true false)
  (`KismetMaterialLibrary.SetScalarParameterValue` "/Game/17_NiagaraEffect/NiagaraSystem/Rain/RainMaterialEffect/MPC_Rain.MPC_Rain" "Rain" 1.0)
  (`LightComponent.SetIntensity` (`self.DirectionalLight`) 4.0))

(fn `SetUnRain`
  (`KismetMaterialLibrary.SetScalarParameterValue` "/Game/07_RainyWeather/MPC_Rainy.MPC_Rainy" "RippleFlatten" 1.0)
  (`ExponentialHeightFogComponent.SetFogDensity` (`self.ExponentialHeightFog`) 0.02)
  (`SceneComponent.SetVisibility` (`self.MS_Rain`) false false)
  (`KismetMaterialLibrary.SetScalarParameterValue` "/Game/17_NiagaraEffect/NiagaraSystem/Rain/RainMaterialEffect/MPC_Rain.MPC_Rain" "Rain")
  (`LightComponent.SetIntensity` (`self.DirectionalLight`) 10.0))

(fn `UserConstructionScript`
  (bind _ms_rain (`self.MS_Rain`))
  (bind _directionallight (`self.DirectionalLight`))
  (bind _exponentialheightfog (`self.ExponentialHeightFog`))
  (`|ExecutionSequence`
    (:`then_0`
      (`SceneComponent.K2_SetWorldRotation` (`self.DirectionalLight`) (`KismetMathLibrary.MakeRotator` 0.0 (`KismetMathLibrary.MapRangeUnclamped` (`self.TimeOfDay`) 600.0 1800.0 180.0 360.0) (`self.SunAngle`)) false false))
    (:`then_1`
      (if (`self.Rainy`)
        (`KismetMaterialLibrary.SetScalarParameterValue` "/Game/07_RainyWeather/MPC_Rainy.MPC_Rainy" "RippleFlatten" 0.0)
        (`ExponentialHeightFogComponent.SetFogDensity` _exponentialheightfog 0.4)
        (`SceneComponent.SetVisibility` _ms_rain true false)
        (`KismetMaterialLibrary.SetScalarParameterValue` "/Game/17_NiagaraEffect/NiagaraSystem/Rain/RainMaterialEffect/MPC_Rain.MPC_Rain" "Rain" 1.0)
        (`LightComponent.SetIntensity` _directionallight 4.0)
        (else
          (`KismetMaterialLibrary.SetScalarParameterValue` "/Game/07_RainyWeather/MPC_Rainy.MPC_Rainy" "RippleFlatten" 1.0)
          (`ExponentialHeightFogComponent.SetFogDensity` _exponentialheightfog 0.02)
          (`SceneComponent.SetVisibility` _ms_rain false false)
          (`KismetMaterialLibrary.SetScalarParameterValue` "/Game/17_NiagaraEffect/NiagaraSystem/Rain/RainMaterialEffect/MPC_Rain.MPC_Rain" "Rain")
          (`LightComponent.SetIntensity` _directionallight 10.0))))))