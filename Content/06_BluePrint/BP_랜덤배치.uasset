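; BP_랜덤배치 (random placement) is an actor that builds a row of copies of one mesh along its local X axis with randomized spacing.
; The construction script loops MashNumber times, adding a static mesh component set to NewMesh.
; Each X position is the index times Distance plus a RandomValue-bounded offset, so jitter grows along the row.
; A stream seeded by InitialSeed keeps layouts repeatable, and the event graph is empty.
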(fn `UserConstructionScript`
  (bind _randomvalue (`self.RandomValue`))
  (set `self.RandomeStream` (`KismetMathLibrary.MakeRandomStream` (`self.Initial Seed`)))
  (for _index (range 1 (+ (`self.MashNumber`) 1))
    (bind _returnvalue (`AddComponent|NODE_AddStaticMeshComponent-0` :`RelativeTransform` (`KismetMathLibrary.MakeTransform` (`KismetMathLibrary.MakeVector` (* _index (+ (`KismetMathLibrary.RandomFloatInRangeFromStream` (`self.RandomeStream`) (* -1.0 _randomvalue) _randomvalue) (`self.Distance`)))))))
    (`StaticMeshComponent.SetStaticMesh` _returnvalue (`self.New Mesh`))))