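; Traffic light actor that endlessly alternates a timed red phase with a green phase showing a two-digit countdown.
; BeginPlay starts a delay-driven event loop that swaps LED materials and toggles matching point lights.
; The counter drops each second, feeding digits into a material "Number" parameter, blanking the leading zero and blinking green for roughly the last ten seconds.
; The construction script previews the initial count through dynamic material instances.
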(event `self.ReceiveBeginPlay`
  (`self.TrafficLightLoop`))

(event `CounterLoop`
  (bind _count (`self.Count`))
  (`self.GreenLight` true :!label _label)
  (`self.CounterLight` true _count)
  (`KismetSystemLibrary.Delay` 0.5)
  (`self.GreenLight` (> _count 10))
  (bind _result (`/Engine/EditorBlueprintResources/StandardMacros.DecrementInt` _count)
    (:`  `
      (bind _output_get (set `self.Count` _result))
      (`KismetSystemLibrary.Delay` 0.5)
      (if (== _output_get 0)
        (set `self.Count` (`self.GreenLightDuration`))
        (`self.TrafficLightLoop`)
        (else
          (`self.CounterLoop`))))))

(event `TrafficLightLoop`
  (`self.InitializeLight`)
  (`self.RedLight` true)
  (`KismetSystemLibrary.Delay` (`self.RedLightDuration`))
  (`self.RedLight` false)
  (set `self.Count` (`self.GreenLightDuration`))
  (goto _label))

(event `InitializeLight`
  (`self.RedLight` false)
  (`self.GreenLight` false)
  (`self.CounterLight` false))

(event `RedLight`
  (params (RedLightOn :type Boolean))
  ;[1 1 1] Red Light
  (`PrimitiveComponent.SetMaterial` (`self.신호등_LEDRed`) 0 (select `bool` RedLightOn :`false` "/Game/09_TrafficLight/M_LED.M_LED" :`true` "/Game/09_TrafficLight/MI_LEDRed_Inst.MI_LEDRed_Inst" :!type "MaterialInterface Object Reference"))
  (`SceneComponent.SetVisibility` (`self.PointLight_Red`) RedLightOn false))

(event `GreenLight`
  (params (GreenLightOn :type Boolean))
  ;[1 1 1] GreenLight
  (`PrimitiveComponent.SetMaterial` (`self.신호등_LEDGreen`) 0 (select `bool` GreenLightOn :`false` "/Game/09_TrafficLight/M_LED.M_LED" :`true` "/Game/09_TrafficLight/MI_LEDGreen_Inst.MI_LEDGreen_Inst" :!type "MaterialInterface Object Reference"))
  (`SceneComponent.SetVisibility` (`self.PointLight_Green`) GreenLightOn false))

(event `CounterLight`
  (params (CounterLightOn :type Boolean) (Count :type Integer))
  (`PrimitiveComponent.SetMaterial` (`self.신호등_숫자10`) 0 (select `bool` CounterLightOn :`false` "/Game/09_TrafficLight/M_LED.M_LED" :`true` "/Game/09_TrafficLight/M_LED_Number.M_LED_Number" :!type "MaterialInterface Object Reference"))
  (`PrimitiveComponent.SetMaterial` (`self.신호등_숫자1`) 0 (select `bool` CounterLightOn :`false` "/Game/09_TrafficLight/M_LED.M_LED" :`true` "/Game/09_TrafficLight/M_LED_Number.M_LED_Number" :!type "MaterialInterface Object Reference"))
  (`SceneComponent.SetVisibility` (`self.PointLight_Count`) CounterLightOn false)
  (if CounterLightOn
    (bind _output_get (set `self.Count` Count))
    (`MeshComponent.SetScalarParameterValueOnMaterials` (`self.신호등_숫자1`) "Number" (`KismetMathLibrary.Conv_IntToDouble` (mod _output_get 10)))
    (`MeshComponent.SetScalarParameterValueOnMaterials` (`self.신호등_숫자10`) "Number" (`KismetMathLibrary.Conv_IntToDouble` (/ _output_get 10)))
    (if (< (`self.Count`) 10)
      (`PrimitiveComponent.SetMaterial` (`self.신호등_숫자10`) 0 "/Game/09_TrafficLight/M_LED.M_LED"))))

(fn `UserConstructionScript`
  (bind _returnvalue (`PrimitiveComponent.CreateDynamicMaterialInstance` (`self.신호등_숫자1`) 0 "/Game/09_TrafficLight/M_LED_Number.M_LED_Number" "None"))
  (`MaterialInstanceDynamic.SetScalarParameterValue` _returnvalue "Number" (`KismetMathLibrary.Conv_IntToDouble` (mod (`self.Count`) 10))) ; 1의자리
  (bind _returnvalue_2 (`PrimitiveComponent.CreateDynamicMaterialInstance` (`self.신호등_숫자10`) 0 (select `bool` (< 9 (`self.Count`)) :`false` "/Game/09_TrafficLight/M_LED.M_LED" :`true` "/Game/09_TrafficLight/M_LED_Number.M_LED_Number" :!type "MaterialInterface Object Reference") "None"))
  (`MaterialInstanceDynamic.SetScalarParameterValue` _returnvalue_2 "Number" (`KismetMathLibrary.Conv_IntToDouble` (/ (`self.Count`) 10))) ; 10의자리
)